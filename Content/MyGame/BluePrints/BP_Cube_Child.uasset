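; Child cube Blueprint for a ball-hitting game that drops a bonus when a gold cube is destroyed.
; At BeginPlay it binds SpawnBonus to OnDestroyed only if the Cube mesh's first material is MI_MetallBase_Gold.
; SpawnBonus spawns BP_Bonus at the cube's location, ignoring collisions.
; BallIsHit runs the parent logic, then prints a debug string; the construction script just calls the parent.
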(event `self.ReceiveBeginPlay`
  (if (== (`PrimitiveComponent.GetMaterial` (`self.Cube`) 0) "/Game/MyGame/Materials/Metalls/MI_MetallBase_Gold.MI_MetallBase_Gold")
    (add `self.OnDestroyed` (delegate `SpawnBonus`))))

(event `SpawnBonus`
  (params (DestroyedActor :type "Actor Object Reference"))
  (`|SpawnActorFromClass` "/Game/MyGame/BluePrints/Bonuses/BP_Bonus.BP_Bonus_C" (`KismetMathLibrary.MakeTransform` (`self.K2_GetActorLocation`)) "AlwaysSpawn" "OverrideRootScale" null null))

(event `self.BallIsHit`
  (`parent.BallIsHit`)
  (`KismetSystemLibrary.PrintString` "Fuck"))

(fn `UserConstructionScript`
  (`parent.UserConstructionScript`))