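; Parent Blueprint for a destructible cube that takes hits from BP_ball and awards score when destroyed.
; The construction script randomly rolls Life from one to three, setting the matching material and Score.
; Each ball hit decrements Life, switching to gold at one remaining, with no material change at two.
; At zero it calls CubeDead with its Score and destroys itself, with leftover debug prints along the way.
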(event `self.ReceiveBeginPlay`)

(event `self.ReceiveHit`
  (params (MyComp :type "PrimitiveComponent Object Reference") (Other :type "Actor Object Reference") (OtherComp :type "PrimitiveComponent Object Reference") (bSelfMoved :type Boolean) (HitLocation :type "Vector Structure") (HitNormal :type "Vector Structure") (NormalImpulse :type "Vector Structure") (Hit :type "HitResult Structure (by ref)"))
  (cast `/Game/MyGame/BluePrints/BP_ball` Other)
  (`self.BallIsHit`)
  (`KismetSystemLibrary.PrintString` "Hello"))

(event `BallIsHit`
  (bind _result (`/Engine/EditorBlueprintResources/StandardMacros.DecrementInt` (`self.Life`))
    (:`  `
      (if (== _result 1)
        (`PrimitiveComponent.SetMaterial` (`self.Cube`) 0 "/Game/MyGame/Materials/Metalls/MI_MetallBase_Gold.MI_MetallBase_Gold")
        (elif (<= _result 0)
          (`self.CubeDead` (`self.Score`))
          (`self.K2_DestroyActor`)
          (`KismetSystemLibrary.PrintString` "DoubleFuck" true true (struct :`G` 0.66 :`B` 1.0 :`A` 1.0) 5.0))))))

(fn `UserConstructionScript`
  (bind _cube (`self.Cube`))
  (bind _output_get (set `self.Life` (`KismetMathLibrary.RandomIntegerInRange` 1 3)))
  (switch `int` _output_get
    (:`1`
      (`PrimitiveComponent.SetMaterial` _cube 0 "/Game/MyGame/Materials/Metalls/MI_MetallBase_Gold.MI_MetallBase_Gold")
      (set `self.Score` 100))
    (:`2`
      (`PrimitiveComponent.SetMaterial` _cube 0 "/Game/MyGame/Materials/Metalls/MI_MetallBase_Silver.MI_MetallBase_Silver")
      (set `self.Score` 150))
    (:`3`
      (`PrimitiveComponent.SetMaterial` _cube 0 "/Engine/VREditor/BasicMeshes/MI_Cube_02.MI_Cube_02")
      (set `self.Score` 200))))