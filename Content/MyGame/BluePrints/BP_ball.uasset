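; BP_ball is a ball actor that moves in a straight line and bounces off whatever it hits.
; Each Tick it sweeps itself along Direction scaled by Speed and delta time, using only the X and Y components.
; On a blocking hit it reflects Direction about the hit normal, raises Speed by AddedSpeed up to a fixed cap, and prints the new speed.
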(event `self.ReceiveTick`
  (params (DeltaSeconds :type "Float (single-precision)"))
  (bind (_returnvalue_x _returnvalue_y) (`KismetMathLibrary.BreakVector` (* (`self.Direction`) (* DeltaSeconds (`self.Speed`)))))
  (bind _sweephitresult (`self.K2_AddActorWorldOffset` (`KismetMathLibrary.MakeVector` _returnvalue_x _returnvalue_y) true))
  (bind (_bblockinghit _binitialoverlap _time _distance _location _impactpoint _normal) (`GameplayStatics.BreakHitResult` _sweephitresult))
  (if _bblockinghit
    (set `self.Direction` (`KismetMathLibrary.GetReflectionVector` (`self.Direction`) _normal))
    (bind _output_get (set `self.Speed` (`KismetMathLibrary.FMin` (+ (`self.Speed`) (`self.AddedSpeed`)) 4000.0)))
    (`KismetSystemLibrary.PrintString` (`KismetStringLibrary.Conv_DoubleToString` _output_get) true true (struct :`G` 0.66 :`B` 1.0 :`A` 1.0) 4.0)))

(fn `UserConstructionScript`)