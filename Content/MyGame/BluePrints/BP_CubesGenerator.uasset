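; BP_CubesGenerator is an actor that displays an editor preview grid of static mesh components, presumably cubes.
; The Construction Script adds X by Y components at Padding intervals along local X and Y and stores them in PreviewArray.
; BeginPlay destroys every stored component, and the graphs spawn nothing to replace them at runtime.
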(event `self.ReceiveBeginPlay`
  (for _array_element (`self.PreviewArray`)
    (`ActorComponent.K2_DestroyComponent` _array_element)))

(fn `UserConstructionScript`
  (for _index (range 1 (+ (`self.X`) 1))
    (for _index_2 (range 1 (+ (`self.Y`) 1))
      (bind _returnvalue (`AddComponent|NODE_AddStaticMeshComponent-0` :`RelativeTransform` (`KismetMathLibrary.MakeTransform` (`KismetMathLibrary.MakeVector` (`KismetMathLibrary.Conv_IntToDouble` (* _index (`self.Padding`))) (`KismetMathLibrary.Conv_IntToDouble` (* _index_2 (`self.Padding`)))))))
      (`KismetArrayLibrary.Array_Add` (`self.PreviewArray`) _returnvalue))))