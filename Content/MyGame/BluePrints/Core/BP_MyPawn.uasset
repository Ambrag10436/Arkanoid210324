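; Player pawn for a ball-and-paddle game that spawns balls, tracks lives and score, and collects bonuses.
; SpawnBall allows one main ball while lives remain; its destruction costs a life, and running out signals game end.
; Cube overlaps with BP_Bonus add score and either widen the Cube until a retriggerable delay resets it, grant a life, or spawn an untracked half-size ball.
; Event dispatchers broadcast life, score and game-end changes.
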(event `self.ReceiveBeginPlay`
  (set `self.DefaultScale` (`SceneComponent.RelativeScale3D` (`self.Cube`))))

(event `SpawnBall`
  (if (not (<= (`self.PlayerLives`) 0))
    (`self.AliveBall`
      (:`then`)
      (:`else`
        (bind _returnvalue (`|SpawnActorFromClass` "/Game/MyGame/BluePrints/BP_ball.BP_ball_C" (`KismetMathLibrary.MakeTransform` (`SceneComponent.K2_GetComponentLocation` (`self.Arrow`))) "Undefined" "OverrideRootScale" null null))
        (bind _output_get (set `self.AliveBall` _returnvalue))
        (add `self.OnDestroyed` _output_get (delegate `BallIsDead`))))))

(event `BallIsDead` :!signature `self.OnDestroyed`
  (params (DestroyedActor :type "Actor Object Reference"))
  (bind _result (`/Engine/EditorBlueprintResources/StandardMacros.DecrementInt` (`self.PlayerLives`))
    (:`  `
      (`self.LivesChanged` _result)
      (if (<= _result 0)
        (`self.GameEnd`)))))

(event `self.Cube.OnComponentBeginOverlap`
  (params (OverlappedComponent :type "PrimitiveComponent Object Reference") (OtherActor :type "Actor Object Reference") (OtherComp :type "PrimitiveComponent Object Reference") (OtherBodyIndex :type Integer) (bFromSweep :type Boolean) (SweepResult :type "HitResult Structure (by ref)"))
  (bind _asbp_bonus (cast `/Game/MyGame/BluePrints/Bonuses/BP_Bonus` OtherActor))
  (switch `/Game/MyGame/BluePrints/Bonuses/E_BonusType` (`/Game/MyGame/BluePrints/Bonuses/BP_Bonus.BonusType` _asbp_bonus)
    (:`NewEnumerator0`
      (`self.MaxEvent`))
    (:`NewEnumerator1`
      (`self.LiveEvent`))
    (:`NewEnumerator2`
      (`self.BallEvent`)))
  (`self.AddedScore` 50)
  (`self.K2_DestroyActor` _asbp_bonus))

(event `MaxEvent`
  (bind _cube (`self.Cube`))
  (bind (_relativescale3d_x _relativescale3d_y _relativescale3d_z) (`KismetMathLibrary.BreakVector` (`SceneComponent.RelativeScale3D` _cube)))
  (`SceneComponent.SetRelativeScale3D` _cube (`KismetMathLibrary.MakeVector` _relativescale3d_x (* _relativescale3d_y 1.5) _relativescale3d_z))
  (`self.MinEvent`))

(event `MinEvent`
  (`KismetSystemLibrary.RetriggerableDelay` 5.0)
  (`SceneComponent.SetRelativeScale3D` (`self.Cube`) (`self.DefaultScale`)))

(event `LiveEvent`
  (bind _result (`/Engine/EditorBlueprintResources/StandardMacros.IncrementInt` (`self.PlayerLives`))
    (:`  `
      (`self.LivesChanged` _result))))

(event `BallEvent`
  (`|SpawnActorFromClass` "/Game/MyGame/BluePrints/BP_ball.BP_ball_C" (`KismetMathLibrary.MakeTransform` (`SceneComponent.K2_GetComponentLocation` (`self.Arrow`)) (struct) (0.5 0.5 0.5)) "Undefined" "OverrideRootScale" null null))

(fn `AddedScore`
  (params (Amount :type Integer))
  (bind _output_get (set `self.AllScore` (+ (`self.AllScore`) (`KismetMathLibrary.Abs_Int` Amount))))
  (`self.ScoreChanged` _output_get))

(fn `UserConstructionScript`)