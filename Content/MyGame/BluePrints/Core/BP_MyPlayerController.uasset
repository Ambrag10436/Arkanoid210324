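; BP_MyPlayerController is a player controller that moves a BP_MyPawn sideways and triggers its ball spawning.
; On possess it caches the pawn as BP_MyPawn, and BeginPlay sets game-only input.
; The Left_Right axis applies a swept, frame-rate-independent Y offset scaled by Speed, and the SpawnBall action calls the pawn's SpawnBall function.
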(event `self.ReceiveBeginPlay`
  (`WidgetBlueprintLibrary.SetInputMode_GameOnly` self))

(event `self.ReceivePossess`
  (params (PossessedPawn :type "Pawn Object Reference"))
  (bind _asbp_my_pawn (cast `/Game/MyGame/BluePrints/Core/BP_MyPawn` PossessedPawn))
  (set `self.MyPawn` _asbp_my_pawn))

(event `InputAxis|Left_Right`
  (params (AxisValue :type "Float (single-precision)"))
  (`self.K2_AddActorWorldOffset` (`self.MyPawn`) (`KismetMathLibrary.MakeVector` 0.0 (* AxisValue (`GameplayStatics.GetWorldDeltaSeconds`) (`self.Speed`))) true false))

(event `InputAction|SpawnBall`
  (params (Key :type "Key Structure"))
  (:`Pressed`
    (`/Game/MyGame/BluePrints/Core/BP_MyPawn.SpawnBall` (`self.MyPawn`))))

(fn `UserConstructionScript`)